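; Enemy character Blueprint that registers itself with MyGameMode's enemy tally on BeginPlay.
; The construction script gives each instance a dynamic material with a random RGB tint set through a vector parameter.
; Die flags the enemy dead, deactivates its movement, notifies the game mode and tells its EnemyAIController to stop detecting the player.
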(event `self.ReceiveBeginPlay`
  (bind _asmy_game_mode (cast `/Game/MyGameMode` (`GameplayStatics.GetGameMode`)))
  (`/Game/MyGameMode.AddNewEnemy` _asmy_game_mode))

(fn `Die`
  (set `self.IsDead` true)
  (`ActorComponent.Deactivate` (`self.CharacterMovement`))
  (bind _asmy_game_mode (cast `/Game/MyGameMode` (`GameplayStatics.GetGameMode`)))
  (`/Game/MyGameMode.EnemyDead` _asmy_game_mode)
  (bind _asenemy_aicontroller (cast `/Game/Enemy/Blueprints/EnemyAIController` (`AIBlueprintHelperLibrary.GetAIController` self)))
  (`/Game/Enemy/Blueprints/EnemyAIController.StopDetectingPlayer` _asenemy_aicontroller))

(fn `UserConstructionScript`
  (bind _returnvalue (`PrimitiveComponent.CreateDynamicMaterialInstance` (`self.Mesh`) 0 "/Game/YBot_Model/YBotModel/EnemyMaterial.EnemyMaterial" "InstanceEnemyMat"))
  (`MaterialInstanceDynamic.SetVectorParameterValue` _returnvalue "ColorVector" (`KismetMathLibrary.Conv_ColorToLinearColor` (make `Color` (`KismetSystemLibrary.MakeLiteralByte` (`KismetMathLibrary.Conv_IntToByte` (`KismetMathLibrary.RandomInteger` 255))) (`KismetSystemLibrary.MakeLiteralByte` (`KismetMathLibrary.Conv_IntToByte` (`KismetMathLibrary.RandomInteger` 255))) (`KismetSystemLibrary.MakeLiteralByte` (`KismetMathLibrary.Conv_IntToByte` (`KismetMathLibrary.RandomInteger` 255)))))))