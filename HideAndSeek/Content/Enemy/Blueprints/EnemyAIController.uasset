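; AI controller for EnemyBP that seeds a blackboard, runs a behavior tree and provides hide-and-flee logic between hiding spots.
; RunToHidingSpot claims the nearest other free spot and moves there, with a timer toggling crouch near low spots.
; On arrival, a looping line-trace check detects the player by view angle and distance, or by hearing range unless crouched.
; Detection triggers a run to another spot, as does a failed move.
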(event `self.ReceiveBeginPlay`
  ;[1 1 1] BeginPlay
  (bind _blackboardcomponent (`self.UseBlackboard` "/Game/BehaviourTree/AIBlackboard.AIBlackboard"))
  (bind _asenemy_bp (cast `/Game/Enemy/Blueprints/EnemyBP` (`self.K2_GetPawn`)))
  (bind _nearesthidingspot (`self.GetNearestHidingSpot` (`/Game/Enemy/Blueprints/EnemyBP.HidingSpots` _asenemy_bp) (`self.K2_GetActorLocation` _asenemy_bp)))
  (`BlackboardComponent.SetValueAsObject` _blackboardcomponent (`self.HidingSpot`) _nearesthidingspot)
  (`BlackboardComponent.SetValueAsEnum` _blackboardcomponent (`self.NewVar_1`) (enumliteral `/Game/BehaviourTree/AIState` "NewEnumerator0"))
  (`self.RunBehaviorTree` "/Game/BehaviourTree/AIBT.AIBT"))

(event `RunToHidingSpot`
  (bind _returnvalue (`self.K2_GetPawn`))
  ;[1 1 1] Correr a un escondite libre
  (`self.StopCheckingLineOfSight`)
  (bind _asenemy_bp (cast `/Game/Enemy/Blueprints/EnemyBP` _returnvalue))
  (bind _myhidingspot (`/Game/Enemy/Blueprints/EnemyBP.MyHidingSpot` _asenemy_bp))
  (`/Engine/EditorBlueprintResources/StandardMacros.IsValid` _myhidingspot
    (:`Is Valid`
      (set `/Game/HidingSpots/HidingSpot.IsOccupied` false _myhidingspot))
    (:`Is Not Valid`
      _))
  (bind _nearesthidingspot (`self.GetNearestHidingSpot` (`/Game/Enemy/Blueprints/EnemyBP.HidingSpots` _asenemy_bp) (`self.K2_GetActorLocation` _returnvalue)))
  (bind _output_get (set `/Game/Enemy/Blueprints/EnemyBP.MyHidingSpot` _nearesthidingspot _asenemy_bp))
  (set `/Game/HidingSpots/HidingSpot.IsOccupied` true _output_get)
  (`|AIMoveTo` (`self.K2_GetPawn`) (0.0 0.0 0.0) _output_get
    (:`then`
      (`/Engine/EditorBlueprintResources/StandardMacros.DoOnce` false :!label _label
        (:`Completed`
          (bind _returnvalue_2 (`KismetSystemLibrary.K2_SetTimer` null "CheckIfShouldCrouch" 0.2 true)))))
    (:`OnSuccess`
      (`|ExecutionSequence`
        (:`then_0`
          (goto _label :!via `Reset`))
        (:`then_1`
          (`KismetSystemLibrary.K2_ClearAndInvalidateTimerHandle` _returnvalue_2))
        (:`then_2`
          (bind _returnvalue_3 (`KismetSystemLibrary.K2_SetTimer` null "PlayerDetection" 0.2 true)))
        (:`then_3`
          (goto _label_2 :!via `Reset`))))
    (:`OnFail`
      (`self.RunToHidingSpot`))))

(event `StopCheckingLineOfSight`
  ;[1 1 1] Correr a un escondite libre
  (`KismetSystemLibrary.K2_ClearAndInvalidateTimerHandle` (stale `RunToHidingSpot` _returnvalue_3)))

(event `PlayerDetection`
  (bind _returnvalue (`self.K2_GetPawn`))
  (bind _returnvalue_2 (`self.K2_GetActorLocation` (`self.K2_GetPawn`)))
  ;[1 1 1] Deteccion del jugador por vista bajo un angulo y por oido si no esta agachado
  (bind _outactors (`GameplayStatics.GetAllActorsOfClass` "/Game/Player/Blueprints/PlayerBP.PlayerBP_C"))
  (bind _returnvalue_3 (`self.K2_GetActorLocation` (`|GetArrayItem` _outactors)))
  (`KismetSystemLibrary.DrawDebugLine` _returnvalue_2 _returnvalue_3 (struct :`R` 1.0 :`B` 0.035352 :`A` 1.0) 0.2 3.0)
  (bind _outactors_2 (`GameplayStatics.GetAllActorsOfClass` "/Game/Enemy/Blueprints/EnemyBP.EnemyBP_C"))
  (bind _outhit (`KismetSystemLibrary.LineTraceSingle` _returnvalue_2 _returnvalue_3 "TraceTypeQuery2" false _outactors_2))
  (bind (_bblockinghit _binitialoverlap _time _distance _location _impactpoint _normal _impactnormal _physmat _hitactor) (`GameplayStatics.BreakHitResult` _outhit))
  (bind _asplayer_bp (cast `/Game/Player/Blueprints/PlayerBP` _hitactor))
  (bind _float (`self.AngleBetweenTwoVectors` (`KismetMathLibrary.GetForwardVector` (`Pawn.GetControlRotation` _returnvalue)) (- _returnvalue_3 _returnvalue_2)))
  (bind _returnvalue_4 (`KismetMathLibrary.Vector_Distance` (`self.K2_GetActorLocation` _returnvalue) _location))
  (if (or (and (<= _float (`self.FieldOfView`)) (<= _returnvalue_4 (`self.SightDistance`))) (and (<= _returnvalue_4 (`self.HearingDistance`)) (not (`Character.bIsCrouched` _asplayer_bp))))
    (`/Engine/EditorBlueprintResources/StandardMacros.DoOnce` false :!label _label_2
      (:`Completed`
        (`self.RunToHidingSpot`)))))

(event `CheckIfShouldCrouch`
  (bind _returnvalue (`self.K2_GetPawn`))
  ;[1 1 1] Comprobacion de si el enemigo debe agacharse al llegar a un escondite
  (bind _asenemy_bp (cast `/Game/Enemy/Blueprints/EnemyBP` _returnvalue))
  (bind _myhidingspot (`/Game/Enemy/Blueprints/EnemyBP.MyHidingSpot` _asenemy_bp))
  (if (and (<= (`KismetMathLibrary.Vector_Distance` (`self.K2_GetActorLocation` _returnvalue) (`self.K2_GetActorLocation` _myhidingspot)) (`self.CrouchingDistance`)) (`/Game/HidingSpots/HidingSpot.IsLow` _myhidingspot))
    (bind _asenemy_bp_2 (cast `/Game/Enemy/Blueprints/EnemyBP` (`self.K2_GetPawn`)))
    (if (not (`Character.bIsCrouched` _asenemy_bp_2))
      (`Character.Crouch` _asenemy_bp_2))
    (else
      (bind _asenemy_bp_3 (cast `/Game/Enemy/Blueprints/EnemyBP` (`self.K2_GetPawn`)))
      (if (`Character.bIsCrouched` _asenemy_bp_3)
        (`Character.UnCrouch` _asenemy_bp_3)))))

(fn `AngleBetweenTwoVectors`
  (params (Angle1 :type "Vector Structure") (Angle2 :type "Vector Structure"))
  (returns (Float :type "Float (double-precision)"))
  (return (`KismetMathLibrary.DegAcos` (`KismetMathLibrary.Dot_VectorVector` Angle1 Angle2))))

(fn `GetNearestHidingSpot`
  (params (HidingSpots :type "Array of /Game/HidingSpots/HidingSpot Object Reference") (ActorLocation :type "Vector Structure"))
  (returns (NearestHidingSpot :type "/Game/HidingSpots/HidingSpot Object Reference"))
  (locals (NearestSpot :type "/Game/HidingSpots/HidingSpot Object Reference") (Distance :type "Float (double-precision)") (EnemyLocation :type "Vector Structure"))
  (set `local.EnemyLocation` ActorLocation)
  (set `local.NearestSpot` (`|GetArrayItem` HidingSpots))
  (set `local.Distance` 10000000000.0)
  (for _array_element HidingSpots
    (bind _asenemy_bp (cast `/Game/Enemy/Blueprints/EnemyBP` (`self.K2_GetPawn`)))
    (if (!= (`/Game/Enemy/Blueprints/EnemyBP.MyHidingSpot` _asenemy_bp) _array_element)
      (if (not (`/Game/HidingSpots/HidingSpot.IsOccupied` _array_element))
        (bind _returnvalue (`KismetMathLibrary.Vector_Distance` (`self.K2_GetActorLocation` _array_element) (`local.EnemyLocation`)))
        (if (and (< _returnvalue (`local.Distance`)) (> _returnvalue 100.0))
          (set `local.Distance` _returnvalue)
          (set `local.NearestSpot` _array_element)))))
  (return (`local.NearestSpot`)))

(fn `StopDetectingPlayer`
  (`self.StopCheckingLineOfSight`))

(fn `UserConstructionScript`)