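; PlayerBP is the player pawn, handling movement, look and crouch toggle input, with jump logic present but unwired.
; Pressing Point sets a Shooting flag that blocks movement; nothing here clears it.
; ShootRays, not called in this graph, spreads parallel horizontal debug-drawn line traces across a width along the actor's yaw, intended to kill the first EnemyBP hit.
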(event `InputAxis|MoveForward`
  (params (AxisValue :type "Float (single-precision)"))
  (if (not (`self.Shooting`))
    (`self.AddMovementInput` (`KismetMathLibrary.GetForwardVector` (`self.GetControlRotation`)) AxisValue)))

(event `InputAxis|MoveRight`
  (params (AxisValue :type "Float (single-precision)"))
  (if (not (`self.Shooting`))
    (`self.AddMovementInput` (`KismetMathLibrary.GetRightVector` (`self.GetControlRotation`)) AxisValue)))

(event `InputAxis|LookSide`
  (params (AxisValue :type "Float (single-precision)"))
  (`self.AddControllerYawInput` AxisValue))

(event `InputAxis|LookUp`
  (params (AxisValue :type "Float (single-precision)"))
  (`self.AddControllerPitchInput` AxisValue))

(event `InputAction|Jump`
  (params (Key :type "Key Structure")))

(event `InputAction|Point`
  (params (Key :type "Key Structure"))
  (:`Pressed`
    (set `self.Shooting` true)))

(event `InputAction|Crouch`
  (params (Key :type "Key Structure"))
  (:`Pressed`
    (if (`self.bIsCrouched`)
      (`self.UnCrouch`)
      (else
        (`self.Crouch`)))))

(fn `ShootRays`
  (params (NumberOfRays :type Integer) (Width :type "Float (double-precision)"))
  (locals (NextRayOffset :type "Float (double-precision)"))
  (bind _returnvalue (+ (* (`self.GetActorRightVector`) (`local.NextRayOffset`)) (`self.K2_GetActorLocation`)))
  (set `local.NextRayOffset` (/ Width 2.0))
  (for _ (range (+ NumberOfRays 1))
    (set `local.NextRayOffset` (- (`local.NextRayOffset`) (/ Width (`KismetMathLibrary.Conv_IntToDouble` NumberOfRays))))
    (bind _outhit (`KismetSystemLibrary.LineTraceSingle` :`Start` _returnvalue :`End` (+ _returnvalue (* (`KismetMathLibrary.GetForwardVector` (`KismetMathLibrary.MakeRotator` 0.0 0.0 (.yaw (`self.K2_GetActorRotation`)))) (`self.PointingDistance`))) :`TraceChannel` "TraceTypeQuery2" :`DrawDebugType` "Persistent"))
    (bind _asenemy_bp (cast `/Game/Enemy/Blueprints/EnemyBP` (`.HitActor` (`GameplayStatics.BreakHitResult` _outhit))))
    (`/Game/Enemy/Blueprints/EnemyBP.Die` _asenemy_bp)
    (break)))

(fn `UserConstructionScript`)